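; BP_MusicBlockManager handles bomb explosion feedback and the slowdown effect in a music-driven game.
; Each tick it polls its state, spawning a particle emitter and playing a sound when a bomb is destroyed.
; While slowdown is active it halves global time dilation and the pitch of the game instance's music player.
; A DoOnce, re-armed during slowdown, restores both once when slowdown ends.
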(event EventTick
  (params (DeltaSeconds :type Float%20%28single-precision%29))
  (|CallParentFunction DeltaSeconds)
  (Utilities|FlowControl|Sequence
    (:then_0
      ;[1 1 1] Handle Bomb Destruction
      (if (Class|MusicBlockManager|WasBombDestroyed)
        (Game|SpawnActorfromClass "/Game/Blueprints/BP_BombParticleEmitter.BP_BombParticleEmitter_C" (Class|MusicBlockManager|GetBombTransform) "Undefined" 0 0)
        (Audio|PlaySound2D "/Game/Sounds/Bomb_Explosion.Bomb_Explosion" 1.0 1.0 0.0 0 0)))
    (:then_1
      ;[1 1 1] Handle Slowdown
      (if (Class|MusicBlockManager|IsSlowdownActive)
        (bind _asto_the_beat_game_instance (Utilities|Casting|CastToToTheBeatGameInstance (Game|GetGameInstance)))
        (Audio|Components|Audio|SetPitchMultiplier (Class|MusicPlayer|GetAudioComponent (Class|TotheBeatGameInstance|GetMusicPlayerInstance _asto_the_beat_game_instance)) 0.5)
        (Utilities|Time|SetGlobalTimeDilation 0.5)
        (goto _label Reset)))
    (:then_2
      (if (not (Class|MusicBlockManager|IsSlowdownActive))
        (Utilities|FlowControl|DoOnce true :!label _label
          (:Completed
            (Audio|Components|Audio|SetPitchMultiplier (Class|MusicPlayer|GetAudioComponent (Class|TotheBeatGameInstance|GetMusicPlayerInstance _asto_the_beat_game_instance)) 1.0)
            (Utilities|Time|SetGlobalTimeDilation 1.0)))))))

(fn ConstructionScript)